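; BP_PreviewEnvironment is a lighting environment actor with a sky light and a directional light, apparently for previewing content.
; Its construction script uses a LightContrast enum with four presets, from low to ultra-high contrast, to set both light intensities.
; Higher contrast dims the sky light and brightens the directional light.
; It also applies the Cubemap variable to the sky light, and its event graph has no active logic.
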(fn `UserConstructionScript`
  (bind _lightcontrast (`self.LightContrast`))
  (`|ExecutionSequence`
    (:`then_0`
      (`SkyLightComponent.SetIntensity` (`self.SkyLight`) (select `/Game/YU_Tool/Environment/Enum_Light` _lightcontrast :`NewEnumerator0` 1.1 :`NewEnumerator1` 0.74 :`NewEnumerator2` 0.38 :`NewEnumerator3` 0.23)))
    (:`then_1`
      (`LightComponent.SetIntensity` (`self.DirectionalLight`) (select `/Game/YU_Tool/Environment/Enum_Light` _lightcontrast :`NewEnumerator0` 3.5 :`NewEnumerator1` 4.0 :`NewEnumerator2` 4.5 :`NewEnumerator3` 5.0)))
    (:`then_2`
      (`SkyLightComponent.SetCubemap` (`self.SkyLight`) (`self.Cubemap`)))))